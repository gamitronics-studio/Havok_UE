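; Havok physics body Blueprint that displays a static mesh and can register its geometry with the physics world.
; The construction script applies CMesh to the Mesh component.
; AddToWorld waits, reads LOD 0 section 0, flattens vertices into X/Y/Z arrays, and passes them with triangles and spawn location to AddMesh.
; BeginPlay is empty, and the binding of AddToWorld to Havok's physics-on event is disconnected.
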(event Custom|AddToWorld
  (bind _z (Variables|Default|GetZ))
  (bind _tri (Variables|Default|GetTri))
  (Utilities|FlowControl|Delay 4.0)
  (Development|PrintString "adding mersh")
  (bind (_vertices _triangles) (Class|KismetProceduralMeshLibrary|GetSectionfromStaticMesh (Variables|Default|GetcMesh)))
  (for _array_element _vertices
    (Utilities|Array|Add (Variables|Default|GetX) (.x _array_element))
    (Utilities|Array|Add (Variables|Default|GetY) (.y _array_element))
    (Utilities|Array|Add (Variables|Default|GetZ) (.z _array_element)))
  (for _array_element_2 _triangles
    (Utilities|Array|Add (Variables|Default|GetTri) _array_element_2))
  (Class|HKBody|AddMesh (Variables|Default|GetX) (Variables|Default|GetY) _z (Utilities|Array|Length _z) _tri (Utilities|Array|Length _tri) (Variables|Default|GetSpawn%20Location)))

(event EventBeginPlay)

(fn ConstructionScript
  (Components|StaticMesh|SetStaticMesh (Variables|Character|GetMesh) (Variables|Default|GetcMesh))
  (|CallParentFunction))