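; BP_HK_Body_Box is a box physics body that registers itself with the HK simulation when play begins.
; BeginPlay passes its dimensions, mass, friction and spawn transform to AddToSimulation, runs the parent BeginPlay, then calls SwitchPhysics with HK.
; AddToSimulation creates the simulated box and scales the mesh to match its length, width and height.
; A Lerp timeline for interpolating actor location is present but never runs.
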(event Custom|AddToSimulation
  (params (L :type Float%20%28single-precision%29) (W :type Float%20%28single-precision%29) (H :type Float%20%28single-precision%29) (Mass :type Float%20%28single-precision%29) (Friction :type Float%20%28single-precision%29) (Location :type Vector) (Quat :type Quat%20Structure))
  (Class|HKBody|CreateBox L W H Mass Friction Location Quat)
  (Transformation|SetWorldScale3D (Variables|Character|GetMesh) (Math|Vector|MakeVector L W H)))

(event EventBeginPlay
  (CallFunction|AddtoSimulation (Variables|Default|GetL) (Variables|Default|GetW) (Variables|Default|GetH) (Variables|Default|GetMass) (Variables|Default|GetFriction) (Variables|Default|GetSpawn%20Location) (Variables|Default|GetSpawn%20Quat))
  (|CallParentFunction)
  (CallFunction|SwitchPhysics (Variables|Default|GetbHK)))

(fn ConstructionScript
  (|CallParentFunction))