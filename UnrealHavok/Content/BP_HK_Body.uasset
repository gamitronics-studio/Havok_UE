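; Physics body actor that switches between Havok simulation and Unreal's built-in physics.
; Binds to the Havok world-cleared event and the UI's HKOn toggle; SwitchPhysics disables mesh physics and collision for Havok, or restores them for Unreal.
; While Havok is active, a gated Tick copies the body's transform to the actor, applying WorldScale, a Y/Z position swap and per-axis rotation conversion.
; The construction script stores SpawnLocation, then scales the actor's position by WorldScale.
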(event Custom|SwitchPhysics
  (params (bHK :type Boolean))
  (bind _mesh (Variables|Default|GetMesh))
  ;[0 0 0 0.8] Switch Physics
  (bind _output_get (Variables|Default|SetbHK bHK))
  (if _output_get
    (Utilities|FlowControl|Sequence
      (:then_0
        (Physics|SetSimulatePhysics _mesh false)
        (Collision|SetCollisionEnabled _mesh "NoCollision"))
      (:then_1
        ;[0 0 0 0.8] Tick: Loc Rot
        (Utilities|FlowControl|Gate true) ; enters at Open
      ))
    (else
      (Utilities|FlowControl|Sequence
        (:then_0
          (Utilities|FlowControl|Gate true) ; enters at Close
        )
        (:then_1
          (Collision|SetCollisionEnabled _mesh "QueryAndPhysics")
          (Physics|SetSimulatePhysics _mesh true))))))

(event EventBeginPlay
  ;[0 0 0 0.8] BeginPlay
  (EventDispatchers|BindEventtoOnWorldCleared (Subsystems|GetHavokSystem) (EventDispatchers|CreateEvent :!event K2DestroyActor))
  (EventDispatchers|BindEventtoHKon (Variables|Default|GetUI) (EventDispatchers|CreateEvent :!event Custom|SwitchPhysics))
  ;[0 0 0 0.8] Tick: Loc Rot
  (Utilities|FlowControl|Gate true) ; enters at Open
)

(event EventTick
  (params (DeltaSeconds :type Float%20%28single-precision%29))
  ;[0 0 0 0.8] Tick: Loc Rot
  (Utilities|FlowControl|Gate true
    (:Exit
      (bind _returnvalue (Class|HKBody|GetLocation))
      (Transformation|SetActorLocation (Math|Vector|MakeVector (.x (* _returnvalue (Variables|Default|GetWorldScale))) (.z (* _returnvalue (Variables|Default|GetWorldScale))) (.y (* _returnvalue (Variables|Default|GetWorldScale)))) true true)
      (bind _returnvalue_2 (Class|HKBody|GetRotation))
      (bind _result (Math|Float|NegateFloat (.roll _returnvalue_2))
        (:%20%20
          (bind _result_2 (Math|Float|NegateFloat (.pitch _returnvalue_2))
            (:%20%20
              (bind _result_3 (Math|Float|NegateFloat (.yaw _returnvalue_2))
                (:%20%20
                  (Transformation|SetActorRotation (Math|Rotator|MakeRotator _result _result_2 _result_3)))))))))))

(fn ConstructionScript
  (Variables|Default|SetSpawn%20Location (Transformation|GetActorLocation))
  (Transformation|SetActorLocation (* (Variables|Default|GetSpawn%20Location) (Variables|Default|GetWorldScale)) false false))