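; Physics manager actor that feeds level geometry into the Havok system and sizes an optional floor.
; It opens the WB_Havok UI and binds to the physics-on event; clearing the world re-adds the floor and triggers re-adds.
; After delays, PhysicsOn registers actors tagged as blocks or statics, plus the first track.
; GetMeshData extracts LOD 0, section 0 triangles for mesh colliders, converting units by 1/40; rotations are negated.
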(event Custom|ClearWorld
  (bind _returnvalue (Subsystems|GetHavokSystem))
  ;[0 0 0 0.8] Clear World
  (Class|HavokSystem|ClearWorld _returnvalue)
  (if (Variables|Default|GetbFloor?)
    (Class|HavokSystem|AddFloor _returnvalue (Variables|Default|GetFloor%20X) (Variables|Default|GetFloor%20Y)))
  (bind _returnvalue_2 (Actor|GetActorOfClass "BP_Physics_C"))
  (Default|CallReAdd _returnvalue_2)
  (CallFunction|Physicson))

(event Custom|PreparePhysics
  ;[0 0 0 0.8] Prepare Physics: UI
  (bind _returnvalue (UserInterface|CreateWidget "/Game/WB_Havok.WB_Havok_C" 0 (Variables|Default|GetFloor%20X) (Variables|Default|GetFloor%20Y) self))
  (UserInterface|Viewport|AddtoViewport _returnvalue 0)
  (Variables|/Script/Engine.PlayerController|SetbShowMouseCursor (Game|GetPlayerController 0) true)
  (EventDispatchers|BindEventtoOnPhysicson (Subsystems|GetHavokSystem) (EventDispatchers|CreateEvent :!event Custom|PhysicsOn)))

(event Custom|PhysicsOn
  ;[0 0 0 0.8] On Phyics On: Add Block Volumes, Statics and Track to World
  (Utilities|FlowControl|Delay 1.0)
  ;;[0 0 0 0.8] Block Volumes
  (bind _outactors (Actor|GetAllActorswithTag "HK Block"))
  (for _array_element _outactors
    (Class|HavokSystem|AddBlock (Subsystems|GetHavokSystem) (.x (* (.scale (Transformation|GetWorldTransform (Variables|/Script/Engine.Actor|GetRootComponent _array_element))) 2.5)) (.z (* (.scale (Transformation|GetWorldTransform (Variables|/Script/Engine.Actor|GetRootComponent _array_element))) 2.5)) (.y (* (.scale (Transformation|GetWorldTransform (Variables|/Script/Engine.Actor|GetRootComponent _array_element))) 2.5)) (/ (.location (Transformation|GetWorldTransform (Variables|/Script/Engine.Actor|GetRootComponent _array_element))) 40) (Math|Conversions|ToQuaternion(Rotator) (Class|KismetMathLibrary|NegateRotator (.rotation (Transformation|GetWorldTransform (Variables|/Script/Engine.Actor|GetRootComponent _array_element)))))))
  ;;[0 0 0 0.8] Statics
  (bind _outactors_2 (Actor|GetAllActorswithTag "HK Static"))
  (for _array_element_2 _outactors_2
    (bind _asstatic_mesh_actor (Utilities|Casting|CastToStaticMeshActor _array_element_2))
    (Utilities|IsValid (Variables|/Script/Engine.StaticMeshComponent|GetStaticMesh (Variables|/Script/Engine.StaticMeshActor|GetStaticMeshComponent _asstatic_mesh_actor))
      (:Is%20Valid
        (Class|HavokSystem|CreateMesh (Subsystems|GetHavokSystem) (.Xs (CallFunction|GetMeshData (Variables|/Script/Engine.StaticMeshComponent|GetStaticMesh (Variables|/Script/Engine.StaticMeshActor|GetStaticMeshComponent _asstatic_mesh_actor)) (.scale (Transformation|GetActorTransform _asstatic_mesh_actor)))) (.Ys (CallFunction|GetMeshData (Variables|/Script/Engine.StaticMeshComponent|GetStaticMesh (Variables|/Script/Engine.StaticMeshActor|GetStaticMeshComponent _asstatic_mesh_actor)) (.scale (Transformation|GetActorTransform _asstatic_mesh_actor)))) (.Zs (CallFunction|GetMeshData (Variables|/Script/Engine.StaticMeshComponent|GetStaticMesh (Variables|/Script/Engine.StaticMeshActor|GetStaticMeshComponent _asstatic_mesh_actor)) (.scale (Transformation|GetActorTransform _asstatic_mesh_actor)))) (.Tris (CallFunction|GetMeshData (Variables|/Script/Engine.StaticMeshComponent|GetStaticMesh (Variables|/Script/Engine.StaticMeshActor|GetStaticMeshComponent _asstatic_mesh_actor)) (.scale (Transformation|GetActorTransform _asstatic_mesh_actor)))) (/ (.location (Transformation|GetActorTransform _asstatic_mesh_actor)) 40) (Math|Conversions|ToQuaternion(Rotator) (Class|KismetMathLibrary|NegateRotator (.rotation (Transformation|GetActorTransform _asstatic_mesh_actor))))))))
  ;;[0 0 0 0.8] Track
  (Utilities|FlowControl|Delay 2.0)
  (bind _outactors_3 (Actor|GetAllActorswithTag "HK Track"))
  (bind _asstatic_mesh_actor_2 (Utilities|Casting|CastToStaticMeshActor (Utilities|Array|Get(acopy) _outactors_3)))
  (Class|HavokSystem|CreateMesh (Subsystems|GetHavokSystem) (.Xs (CallFunction|GetMeshData (Variables|/Script/Engine.StaticMeshComponent|GetStaticMesh (Variables|/Script/Engine.StaticMeshActor|GetStaticMeshComponent _asstatic_mesh_actor_2)) (.scale (Transformation|GetActorTransform _asstatic_mesh_actor_2)))) (.Ys (CallFunction|GetMeshData (Variables|/Script/Engine.StaticMeshComponent|GetStaticMesh (Variables|/Script/Engine.StaticMeshActor|GetStaticMeshComponent _asstatic_mesh_actor_2)) (.scale (Transformation|GetActorTransform _asstatic_mesh_actor_2)))) (.Zs (CallFunction|GetMeshData (Variables|/Script/Engine.StaticMeshComponent|GetStaticMesh (Variables|/Script/Engine.StaticMeshActor|GetStaticMeshComponent _asstatic_mesh_actor_2)) (.scale (Transformation|GetActorTransform _asstatic_mesh_actor_2)))) (.Tris (CallFunction|GetMeshData (Variables|/Script/Engine.StaticMeshComponent|GetStaticMesh (Variables|/Script/Engine.StaticMeshActor|GetStaticMeshComponent _asstatic_mesh_actor_2)) (.scale (Transformation|GetActorTransform _asstatic_mesh_actor_2)))) (/ (.location (Transformation|GetActorTransform _asstatic_mesh_actor_2)) 40) (Math|Conversions|ToQuaternion(Rotator) (Class|KismetMathLibrary|NegateRotator (.rotation (Transformation|GetActorTransform _asstatic_mesh_actor_2))))))

(event Custom|SetFloor
  ;[0 0 0 0.8] Set Floor
  (Transformation|SetWorldScale3D (Variables|Default|GetFloor) (Math|Vector|MakeVector (* (Variables|Default|GetFloor%20X) 0.8) (* (Variables|Default|GetFloor%20Y) 0.8) 0.5))
  (Rendering|SetActorHiddenInGame (not (Variables|Default|GetbFloor?))))

(fn ConstructionScript
  (Transformation|SetWorldScale3D (Variables|Default|GetFloor) (Math|Vector|MakeVector (* (Variables|Default|GetFloor%20X) 0.8) (* (Variables|Default|GetFloor%20Y) 0.8) 0.5))
  (Rendering|SetActorHiddenInGame (not (Variables|Default|GetbFloor?))))

(fn GetMeshData
  (params (Mesh :type Static%20Mesh%20Object%20Reference) (Scale :type Vector))
  (bind (_vertices _triangles) (Class|KismetProceduralMeshLibrary|GetSectionfromStaticMesh Mesh))
  (for _array_element _vertices
    (Utilities|Array|Add (LocalVariables|GetX) (/ (* (.x Scale) (.x _array_element)) 4e+01))
    (Utilities|Array|Add (LocalVariables|GetY) (/ (* (.y Scale) (.y _array_element)) 4e+01))
    (Utilities|Array|Add (LocalVariables|GetZ) (/ (* (.z Scale) (.z _array_element)) 4e+01)))
  (for _array_element_2 _triangles
    (Utilities|Array|Add (LocalVariables|GetTri) _array_element_2))
  (return (LocalVariables|GetX) (LocalVariables|GetY) (LocalVariables|GetZ) (LocalVariables|GetTri)))