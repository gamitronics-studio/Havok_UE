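; Block actor that registers its mesh as a block in a Havok physics system.
; On BeginPlay it binds AddToWorld to the Havok system's OnPhysicsOn event and to ReAdd on the BP_Physics actor.
; AddToWorld waits briefly, then calls AddBlock with the mesh transform converted for Havok: Y/Z-swapped scale, scaled-down location and negated rotation as a quaternion.
; It prints a debug message after each add.
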(event Custom|AddToWorld
  (bind _mesh (Variables|Default|GetMesh))
  (bind _returnvalue (Transformation|GetWorldTransform _mesh))
  (bind _returnvalue_2 (* (.scale _returnvalue) 1))
  (Utilities|FlowControl|Delay 0.2)
  (Class|HavokSystem|AddBlock (Subsystems|GetHavokSystem) (.x _returnvalue_2) (.z _returnvalue_2) (.y _returnvalue_2) (/ (.location _returnvalue) 40) (Math|Conversions|ToQuaternion(Rotator) (Class|KismetMathLibrary|NegateRotator (.rotation _returnvalue))))
  (Development|PrintString "Added"))

(event EventBeginPlay
  (EventDispatchers|BindEventtoOnPhysicson (Subsystems|GetHavokSystem) (delegate Custom|AddToWorld))
  (bind _returnvalue (Actor|GetActorOfClass "/Game/BP_Physics.BP_Physics_C"))
  (EventDispatchers|BindEventtoReAdd _returnvalue (delegate Custom|AddToWorld)))

(fn ConstructionScript)