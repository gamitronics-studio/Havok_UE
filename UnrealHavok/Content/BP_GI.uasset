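; Game instance that persists car profiles across sessions and shuts down the Havok physics system on exit.
; Init asynchronously loads the CarProfiles save slot or creates an initial BP_Save, and SaveCar writes the current profiles back to it.
; Shutdown stops physics, then calls quit after a one-second delay.
; Other Havok calls, including physics start and world building, are left unconnected and never run.
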(event Custom|Load%20Car%20Saves
  ;[0 0 0 0.8] Save System
  ;;[0 0 0 0.8] load saved Cars
  (bind _returnvalue (SaveGame|DoesSaveGameExist "CarProfiles"))
  (if _returnvalue
    (bind _savegame (|AsyncLoadGamefromSlot "CarProfiles")
      (:Completed
        (bind _asbp_save (Utilities|Casting|CastToBP_Save _savegame))
        (bind _output_get (Variables|Default|SetSaveObj _asbp_save))
        (Variables|Default|SetCar%20Profiles (Variables|/Game/BP_Save.BP_Save_C|GetCarProfiles _output_get))
        (Development|PrintString "Profiles Loaded")))
    (else
      (bind _returnvalue_2 (SaveGame|CreateSaveGameObject "/Game/BP_Save.BP_Save_C"))
      (Variables|Default|SetSaveObj _returnvalue_2)
      (|AsyncSaveGametoSlot self (Variables|Default|GetSaveObj) "CarProfiles"
        (:then
          (Development|PrintString "Save: creating initial save"))
        (:Completed
          (Development|PrintString "Profiles Saveed"))))))

(event Custom|Save%20Car
  (bind _saveobj (Variables|Default|GetSaveObj))
  ;[0 0 0 0.8] Save System
  ;;[0 0 0 0.8] Save
  (Utilities|IsValid _saveobj
    (:Is%20Valid
      (Variables|/Game/BP_Save.BP_Save_C|SetCarProfiles _saveobj (Variables|Default|GetCar%20Profiles))
      (|AsyncSaveGametoSlot self (Variables|Default|GetSaveObj) "CarProfiles"
        (:Completed
          (Development|PrintString "Profiles Saveed"))))))

(event EventShutdown
  (bind _returnvalue (Subsystems|GetHavokSystem))
  ;[0 0 0 0.8] Shutdown: Physics Stop and Quit
  (Class|HavokSystem|PhysicsStop _returnvalue)
  (Utilities|FlowControl|Delay 1.0)
  (Class|HavokSystem|PhysicsQuit _returnvalue)
  (Development|PrintString "Quited"))

(event EventInit
  ;[0 0 0 0.8] Init: load saved Car profiles
  (Development|PrintString "GU: inited")
  (CallFunction|LoadCarSaves))