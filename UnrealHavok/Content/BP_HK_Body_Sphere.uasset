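; BP_HK_Body_Sphere is a sphere body actor for the custom HK physics simulation.
; On BeginPlay it calls AddToSimulation, which creates the sphere from radius, mass, friction and spawn location, then multiplies the mesh's world scale by the radius.
; The parent BeginPlay runs after registration.
; A physics switch call and a timeline that lerps actor location are present but unconnected, so neither runs.
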(event Custom|AddToSimulation
  (params (Radius :type Float%20%28single-precision%29) (Mass :type Float%20%28single-precision%29) (Friction :type Float%20%28single-precision%29) (SpawnLocation :type Vector))
  (bind _mesh (Variables|Character|GetMesh))
  (Class|HKBody|CreateSphere Radius Mass Friction SpawnLocation)
  (Transformation|SetWorldScale3D _mesh (* (Transformation|GetWorldScale _mesh) Radius)))

(event EventBeginPlay
  (CallFunction|AddtoSimulation (Variables|Default|GetRadius) (Variables|Default|GetMass) (Variables|Default|GetFriction) (Variables|Default|GetSpawn%20Location))
  (|CallParentFunction))

(fn ConstructionScript
  (|CallParentFunction))