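; Player car pawn driven by a Havok vehicle simulation, with a HUD, handbrake, reset, camera rotation and boost.
; BuildAndStart lays out wheels and suspension from SetupData, spawns the simulated car from static mesh triangles scaled down by 40, then opens the Tick gate.
; Each tick steps the simulation with input, then copies location (times 40), rotation, wheel spin and stats back to the actor.
; Boost swaps setups stored in BP_GI.
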(event Custom|BuildAndStart
  (bind _carmesh (Variables|Default|GetCarMesh))
  (bind _t_fr (Variables|Default|GetT_FR))
  (bind _returnvalue (Transformation|GetWorldScale _t_fr))
  (bind _returnvalue_2 (Transformation|GetWorldScale _carmesh))
  (bind _staticmesh (Variables|/Script/Engine.StaticMeshComponent|GetStaticMesh _t_fr))
  (bind _staticmesh_2 (Variables|/Script/Engine.StaticMeshComponent|GetStaticMesh _carmesh))
  (bind (_xs _ys _zs _tris) (CallFunction|GetMeshData _staticmesh _returnvalue))
  (bind (_xs_2 _ys_2 _zs_2 _tris_2) (CallFunction|GetMeshData _staticmesh_2 _returnvalue_2))
  ;[0 0 0 0.5] BuildAndStart: Show mesh, SpawnCar, HUD, Start Tick update
  (Development|SetHiddeninGame (Variables|Default|GetCarMesh) false true)
  (CallFunction|PrintSetup)
  (CallFunction|SetWheels)
  (Class|HKVehicle|SpawnCar (Variables|Default|GetSetup%20Data) _xs_2 _ys_2 _zs_2 _tris_2 (Utilities|Struct|MakeMeshData _xs _ys _zs _tris))
  (Utilities|FlowControl|Sequence
    (:then_0
      (bind _returnvalue_3 (UserInterface|CreateWidget "/Game/WB_Car.WB_Car_C" 0 self))
      (Variables|Default|SetWB_HUD _returnvalue_3)
      (UserInterface|Viewport|AddtoViewport (Variables|Default|GetWB_HUD) 0))
    (:then_1
      (CallFunction|OpenTick)
      (bind _returnvalue_4 (Class|HKVehicle|GetCatSetup))
      (Development|PrintString (Utilities|String|ToString(Text) (Utilities|Text|FormatText "(post setup) 
Mass: {mass} 
Max Speed: {speed} 
Torque: {Torque} 
Min RPM: {minRPM} 
Max RPM: {maxRPM} 
Opt RPM: {optRPM} 
Down RPM: {dRPM} 
Up RPM: {uRPM} 
Reverse G: {RG} 
Steer Angle: {angle} 
Lift Coefficient: {lc} 
RT Wheels: {bRT}  
Custom Body: {bCB} 
 
Wheel Radius: {WR} 
Wheel Thickness: {WT} 
Suspension Length: {SL} 
Custom Wheel: {bCW}" 0 0 0 0 0 0 0 0 0 0 0 (.bUseRayTrace (Utilities|Struct|BreakCarSetup _returnvalue_4)) 0 0 0 0 (.bUseCustomWheel (Utilities|Struct|BreakCarSetup _returnvalue_4))))))))

(event Custom|Input
  ;[0 0 0 0.5] Update State
  (Class|HKVehicle|StepCar (Variables|Default|GetA) (Variables|Default|GetS) (Variables|Default|GetR) (Variables|Default|GetB) 0.0)
  (Utilities|FlowControl|Sequence
    (:then_0
      ;[0 0 0 0.5] Location Update
      (bind _returnvalue (Class|HKVehicle|GetCarLoc))
      (bind _output_get (Variables|Default|SetEngine%20Location _returnvalue))
      (Transformation|SetActorLocation (* _output_get "40.000000,40.000000,40.000000") false false))
    (:then_1
      ;[0 0 0 0.5] Rotation update
      (bind _returnvalue_2 (Class|HKVehicle|GetCarRot))
      (Transformation|SetActorRotation (* _returnvalue_2 -1.0))
      ;[0 0 0 0.5] Wheels Update
      (bind (_t1l _t1q _t2l _t2q _t3l _t3q _t4l _t4q) (Class|HKVehicle|UpdateWheels))
      (Utilities|FlowControl|Sequence
        (:then_0
          (Transformation|SetRelativeRotation (Variables|Default|GetT_FR) (Math|Rotator|MakeRotator 9e+01 (* (.yaw (Class|KismetMathLibrary|QuatRotator _t1q)) -1.0) 0.0) false false)
          (Transformation|SetRelativeRotation (Variables|Default|GetArrow_FR) (Math|Rotator|MakeRotator 0.0 0.0 (Variables|Default|GetAngle)) false false))
        (:then_1
          (Transformation|SetRelativeRotation (Variables|Default|GetT_FL) (Math|Rotator|MakeRotator 9e+01 (* (.yaw (Class|KismetMathLibrary|QuatRotator _t2q)) -1.0) 0.0) false false)
          (Transformation|SetRelativeRotation (Variables|Default|GetArrow_FL) (Math|Rotator|MakeRotator 0.0 0.0 (Variables|Default|GetAngle)) false false))
        (:then_2
          (Transformation|SetRelativeRotation (Variables|Default|GetT_BL) (Math|Rotator|MakeRotator 9e+01 (* (.Yaw (Math|Rotator|BreakRotator (Class|KismetMathLibrary|QuatRotator _t3q))) -1.0) 0.0) false false)
          (Transformation|SetRelativeRotation (Variables|Default|GetT_BR) (Math|Rotator|MakeRotator 9e+01 (* (.Yaw (Math|Rotator|BreakRotator (Class|KismetMathLibrary|QuatRotator _t4q))) -1.0) 0.0) false false))))
    (:then_2
      ;[0 0 0 0.5] Stats
      (bind (_rpm _kmph _gear _isreverse _torque _steerangle) (Class|HKVehicle|GetCarStats))
      (Variables|Default|SetRPM _rpm)
      (Variables|Default|SetKMPH _kmph)
      (Variables|Default|SetGear _gear)
      (Variables|Default|SetisReverse _isreverse)
      (Variables|Default|SetTorque (Math|Float|Truncate _torque))
      (Variables|Default|SetSteerAngle _steerangle))))

(event Custom|SetWheels
  (bind _setup_data (Variables|Default|GetSetup%20Data))
  (bind _setup_data_2 (Variables|Default|GetSetup%20Data))
  (bind (_suspensionlength _u _f _b _l) (Utilities|Struct|BreakCarSetup _setup_data))
  (bind (_wheelradius _wheelthickness _suspensionlength_2 _u_2 _f_2 _b_2 _l_2) (Utilities|Struct|BreakCarSetup _setup_data_2))
  (bind _returnvalue (* _u -4e+01))
  (bind _returnvalue_2 (* _l -45.0))
  (bind _returnvalue_3 (* _f 4e+01))
  (bind _returnvalue_4 (* _b -4e+01))
  (bind _returnvalue_5 (* _l 45.0))
  (bind _returnvalue_6 (* _u_2 -4e+01))
  (bind _returnvalue_7 (* _f_2 4e+01))
  (bind _returnvalue_8 (* _b_2 -4e+01))
  (bind _returnvalue_9 (* _l_2 4e+01))
  (bind _returnvalue_10 (* _l_2 -4e+01))
  (bind _returnvalue_11 (* _suspensionlength_2 -4e+01))
  (bind _returnvalue_12 (+ _returnvalue_6 _returnvalue_11))
  ;[0 0 0 0.8] Set Wheels
  (Transformation|SetWorldScale3D (Variables|Default|GetT_FR) (Math|Vector|MakeVector (* 0.75 _wheelradius) (* 0.75 _wheelradius) (* 0.5 _wheelthickness)))
  (Utilities|FlowControl|Sequence
    (:then_0
      (Transformation|SetRelativeLocation (Variables|Default|GetArrow_FR) (Math|Vector|MakeVector _returnvalue_7 _returnvalue_9 _returnvalue_12) false false)
      (Transformation|SetRelativeLocation (Variables|Default|GetArrow_FL) (Math|Vector|MakeVector _returnvalue_7 _returnvalue_10 _returnvalue_12) false false))
    (:then_1
      (Transformation|SetRelativeLocation (Variables|Default|GetT_BR) (Math|Vector|MakeVector _returnvalue_8 _returnvalue_9 _returnvalue_12) false false)
      (Transformation|SetRelativeLocation (Variables|Default|GetT_BL) (Math|Vector|MakeVector _returnvalue_8 _returnvalue_10 _returnvalue_12) false false))
    (:then_2
      (Transformation|SetWorldScale3D (Variables|Default|GetSP_BL) (Math|Vector|MakeVector _suspensionlength 1.0 1.0))
      (Transformation|SetRelativeLocation (Variables|Default|GetSP_FR) (Math|Vector|MakeVector _returnvalue_3 _returnvalue_5 _returnvalue) false false)
      (Transformation|SetRelativeLocation (Variables|Default|GetSP_FL) (Math|Vector|MakeVector _returnvalue_3 _returnvalue_2 _returnvalue) false false)
      (Transformation|SetRelativeLocation (Variables|Default|GetSP_BR) (Math|Vector|MakeVector _returnvalue_4 _returnvalue_5 _returnvalue) false false)
      (Transformation|SetRelativeLocation (Variables|Default|GetSP_BL) (Math|Vector|MakeVector _returnvalue_4 _returnvalue_2 _returnvalue) false false))))

(event Custom|OpenTick
  ;[0 0 0 0.5] Tick
  (Utilities|FlowControl|Gate true) ; enters at Open
)

(event EventBeginPlay
  (bind _returnvalue (Game|GetPlayerController 0))
  ;[0 0 0 0.5] BeginPlay: Enable Input, Camera | Hide Mesh | Bind Havok WorldCleared
  (EventDispatchers|BindEventtoOnWorldCleared (Subsystems|GetHavokSystem) (EventDispatchers|CreateEvent :!event K2DestroyActor))
  (Development|SetHiddeninGame (Variables|Default|GetCarMesh) true true)
  (Input|EnableInput _returnvalue)
  (Game|Player|SetViewTargetwithBlend _returnvalue self 0.0 "VTBlend_Linear" 0.0 false))

(event EventTick
  (params (DeltaSeconds :type Float%20%28single-precision%29))
  ;[0 0 0 0.5] Tick
  (Utilities|FlowControl|Gate true
    (:Exit
      ;[0 0 0 0.5] Update State
      (Class|HKVehicle|StepCar (Variables|Default|GetA) (Variables|Default|GetS) (Variables|Default|GetR) (Variables|Default|GetB) 0.0)
      (Utilities|FlowControl|Sequence
        (:then_0
          ;[0 0 0 0.5] Location Update
          (bind _returnvalue (Class|HKVehicle|GetCarLoc))
          (bind _output_get (Variables|Default|SetEngine%20Location _returnvalue))
          (Transformation|SetActorLocation (* _output_get "40.000000,40.000000,40.000000") false false))
        (:then_1
          ;[0 0 0 0.5] Rotation update
          (bind _returnvalue_2 (Class|HKVehicle|GetCarRot))
          (Transformation|SetActorRotation (* _returnvalue_2 -1.0))
          ;[0 0 0 0.5] Wheels Update
          (bind (_t1l _t1q _t2l _t2q _t3l _t3q _t4l _t4q) (Class|HKVehicle|UpdateWheels))
          (Utilities|FlowControl|Sequence
            (:then_0
              (Transformation|SetRelativeRotation (Variables|Default|GetT_FR) (Math|Rotator|MakeRotator 9e+01 (* (.yaw (Class|KismetMathLibrary|QuatRotator _t1q)) -1.0) 0.0) false false)
              (Transformation|SetRelativeRotation (Variables|Default|GetArrow_FR) (Math|Rotator|MakeRotator 0.0 0.0 (Variables|Default|GetAngle)) false false))
            (:then_1
              (Transformation|SetRelativeRotation (Variables|Default|GetT_FL) (Math|Rotator|MakeRotator 9e+01 (* (.yaw (Class|KismetMathLibrary|QuatRotator _t2q)) -1.0) 0.0) false false)
              (Transformation|SetRelativeRotation (Variables|Default|GetArrow_FL) (Math|Rotator|MakeRotator 0.0 0.0 (Variables|Default|GetAngle)) false false))
            (:then_2
              (Transformation|SetRelativeRotation (Variables|Default|GetT_BL) (Math|Rotator|MakeRotator 9e+01 (* (.Yaw (Math|Rotator|BreakRotator (Class|KismetMathLibrary|QuatRotator _t3q))) -1.0) 0.0) false false)
              (Transformation|SetRelativeRotation (Variables|Default|GetT_BR) (Math|Rotator|MakeRotator 9e+01 (* (.Yaw (Math|Rotator|BreakRotator (Class|KismetMathLibrary|QuatRotator _t4q))) -1.0) 0.0) false false))))
        (:then_2
          ;[0 0 0 0.5] Stats
          (bind (_rpm _kmph _gear _isreverse _torque _steerangle) (Class|HKVehicle|GetCarStats))
          (Variables|Default|SetRPM _rpm)
          (Variables|Default|SetKMPH _kmph)
          (Variables|Default|SetGear _gear)
          (Variables|Default|SetisReverse _isreverse)
          (Variables|Default|SetTorque (Math|Float|Truncate _torque))
          (Variables|Default|SetSteerAngle _steerangle))))))

(event EventDestroyed
  ;[0 0 0 0.5] OnDestroy: remove HUD
  (Variables|Default|SetWB_HUD 0))

(event Input|ActionEvents|InputActionHandBrake
  (params (Key :type Key%20Structure :default "None"))
  ;[0 0 0 0.5] Inputs
  (:Pressed
    (Variables|Default|SetB true))
  (:Released
    (Variables|Default|SetB false)))

(event Input|ActionEvents|InputActionCamera
  (params (Key :type Key%20Structure :default "None"))
  (bind _springarm (Variables|Default|GetSpringArm))
  (bind _returnvalue (Transformation|GetWorldRotation _springarm))
  ;[0 0 0 0.5] C: Change Camera
  (:Released
    (Transformation|SetRelativeRotation _springarm (Math|Rotator|MakeRotator (.roll _returnvalue) (.pitch _returnvalue) (+ (.yaw _returnvalue) 9e+01)) false false)))

(event Input|ActionEvents|InputActionResetCar
  (params (Key :type Key%20Structure :default "None"))
  ;[0 0 0 0.5] R: Reset Car Loc
  (:Released
    (Class|HKVehicle|ResetCar)))

(event Input|ActionEvents|InputActionBoost
  (params (Key :type Key%20Structure :default "None"))
  (bind _returnvalue (Game|GetGameInstance))
  (bind _asbp_gi (Utilities|Casting|CastToBP_GI _returnvalue))
  ;[0 0 0 0.8] Boost
  (:Pressed
    (Class|HKVehicle|UpdateCar (Variables|/Game/BP_GI.BP_GI_C|GetBoostSetup _asbp_gi)))
  (:Released
    (Class|HKVehicle|UpdateCar (Variables|/Game/BP_GI.BP_GI_C|GetLastCarSetup _asbp_gi))))

(event Input|AxisEvents|InputAxisMove
  (params (AxisValue :type Float%20%28single-precision%29))
  ;[0 0 0 0.5] Inputs
  (Variables|Default|SetA AxisValue))

(event Input|AxisEvents|InputAxisSteer
  (params (AxisValue :type Float%20%28single-precision%29))
  (bind _setup_data (Variables|Default|GetSetup%20Data))
  (bind _maxsteer (Utilities|Struct|BreakCarSetup _setup_data))
  ;[0 0 0 0.5] Inputs
  (bind _output_get (Variables|Default|SetS AxisValue))
  (Variables|Default|SetAngle (Math|Float|MapRangeClamped _output_get -1.0 1.0 (* _maxsteer -1.0) _maxsteer)))

(fn ConstructionScript)

(fn PrintSetup
  (bind _setup_data (Variables|Default|GetSetup%20Data))
  (Development|PrintText (Utilities|Text|FormatText "Mass: {mass} 
Max Speed: {speed} 
Torque: {Torque} 
Min RPM: {minRPM} 
Max RPM: {maxRPM} 
Opt RPM: {optRPM} 
Down RPM: {dRPM} 
Up RPM: {uRPM} 
Reverse G: {RG} 
Steer Angle: {angle} 
Lift Coefficient: {lc} 
RT Wheels: {bRT}  
Custom Body: {bCB} 
 
Wheel Radius: {WR} 
Wheel Thickness: {WT} 
Suspension Length: {SL} 
Custom Wheel: {bCW}" (.mass _setup_data) (.maxspeed _setup_data) (.torque _setup_data) (.minrpm _setup_data) (.maxrpm _setup_data) (.optrpm _setup_data) (.downshiftatrpm _setup_data) (.upshiftatrpm _setup_data) (.reversegearratio _setup_data) (.maxsteer _setup_data) (.liftcoefficient _setup_data) (.buseraytrace _setup_data) (.busecustomcar _setup_data) (.wheelradius _setup_data) (.wheelthickness _setup_data) (.suspensionlength _setup_data) (.busecustomwheel _setup_data))))

(fn GetMeshData
  (params (Mesh :type Static%20Mesh%20Object%20Reference) (Scale :type Vector))
  (bind (_vertices _triangles) (Class|KismetProceduralMeshLibrary|GetSectionfromStaticMesh Mesh))
  (for _array_element _vertices
    (Utilities|Array|Add (LocalVariables|GetX) (/ (* (.x Scale) (.x _array_element)) 4e+01))
    (Utilities|Array|Add (LocalVariables|GetY) (/ (* (.y Scale) (.y _array_element)) 4e+01))
    (Utilities|Array|Add (LocalVariables|GetZ) (/ (* (.z Scale) (.z _array_element)) 4e+01)))
  (for _array_element_2 _triangles
    (Utilities|Array|Add (LocalVariables|GetTri) _array_element_2))
  (return (LocalVariables|GetX) (LocalVariables|GetY) (LocalVariables|GetZ) (LocalVariables|GetTri)))