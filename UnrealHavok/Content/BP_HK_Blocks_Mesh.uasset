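; A block actor that registers its static mesh as a triangle mesh in a custom Havok physics system.
; On the system's physics-on event or a BP_Physics re-add event, it waits briefly, then reads vertices and triangles from CMesh's first LOD and section.
; These feed CreateMesh with the location, both downscaled by 40; rotation and scale are not passed.
; The arrays are not cleared between re-adds, so geometry accumulates.
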(event Custom|AddToWorld
  (Utilities|FlowControl|Delay 0.2)
  (CallFunction|Meshed)
  (Class|HavokSystem|CreateMesh (Subsystems|GetHavokSystem) (Variables|Default|GetX) (Variables|Default|GetY) (Variables|Default|GetZ) (Variables|Default|GetTri) (/ (.location (Transformation|GetWorldTransform (Variables|Default|GetMesh))) 40))
  (Development|PrintString "Added"))

(event Custom|Meshed
  (Development|PrintString "adding mersh")
  (bind (_vertices _triangles) (Class|KismetProceduralMeshLibrary|GetSectionfromStaticMesh (Variables|Default|GetcMesh)))
  (for _array_element _vertices
    (Utilities|Array|Add (Variables|Default|GetX) (/ (.x _array_element) 4e+01))
    (Utilities|Array|Add (Variables|Default|GetY) (/ (.y _array_element) 4e+01))
    (Utilities|Array|Add (Variables|Default|GetZ) (/ (.z _array_element) 4e+01)))
  (for _array_element_2 _triangles
    (Utilities|Array|Add (Variables|Default|GetTri) _array_element_2)))

(event EventBeginPlay
  (EventDispatchers|BindEventtoOnPhysicson (Subsystems|GetHavokSystem) (delegate Custom|AddToWorld))
  (bind _returnvalue (Actor|GetActorOfClass "/Game/BP_Physics.BP_Physics_C"))
  (EventDispatchers|BindEventtoReAdd _returnvalue (delegate Custom|AddToWorld)))

(fn ConstructionScript
  (Components|StaticMesh|SetStaticMesh (Variables|Default|GetMesh) (Variables|Default|GetcMesh))
  (|CallParentFunction))